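; NPC character Blueprint for AI combatants that handles death and exposes targeting, team and attack state.
; When its health component depletes, it ragdolls the mesh from the pelvis bone down and returns its tokens to the Blackboard target actor.
; The same Blackboard target supplies the shoot location, the team tag is fixed to NPC, and the armed check mirrors the attacking flag.
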(event `self.ReceiveActorBeginOverlap`
  (params (OtherActor :type "Actor Object Reference")))

(event `self.HealthComponent.OnHealthDepleted`
  (params (DamageCauser :type "Actor Object Reference"))
  (bind _pelvisbonename (`self.PelvisBoneName`))
  (bind _mesh (`self.Mesh`))
  (`PrimitiveComponent.SetCollisionProfileName` (`self.Mesh`) "Ragdoll" true)
  (`SkeletalMeshComponent.SetAllBodiesBelowSimulatePhysics` _mesh _pelvisbonename true true)
  (`SkeletalMeshComponent.SetAllBodiesBelowPhysicsBlendWeight` _mesh _pelvisbonename 1.0 false true)
  (set `self.InRagdoll` true)
  (`self.Return Tokens`))

(event `self.ReceiveTick`
  (params (DeltaSeconds :type "Float (single-precision)")))

(event `self.ReceiveBeginPlay`)

(fn `Get Shoot Target Location`
  (returns (Location :type "Vector Structure"))
  (bind _asactor (cast `Actor` (`BlackboardComponent.GetValueAsObject` (`AIBlueprintHelperLibrary.GetBlackboard` null) (`self.TargetActorKey`)))
    (:`then`
      (return (`self.K2_GetActorLocation` _asactor)))
    (:`CastFailed`
      (`KismetSystemLibrary.PrintString` "target not found")
      (return (0.0 0.0 0.0)))))

(fn `GetTeamTag`
  (returns (ReturnValue :type "GameplayTag Structure"))
  (return (struct :`TagName` "Character.NPC")))

(fn `IsArmed`
  (returns (ReturnValue :type Boolean))
  (return (`self.Is Attacking`)))

(fn `IsAttacking`
  (returns (IsAttacking :type Boolean))
  (return (`self.Is Attacking`)))

(fn `Return Tokens`
  (bind _asactor (cast `Actor` (`BlackboardComponent.GetValueAsObject` (`AIBlueprintHelperLibrary.GetBlackboard` null) (`self.TargetActorKey`)))
    (:`then`
      (bind _returnvalue (message `AITarget.ReturnTokens` _asactor self))
      (if (not _returnvalue)
        (`KismetSystemLibrary.PrintString` "no tokens returned" :!label _label)))
    (:`CastFailed`
      (goto _label))))

(fn `UserConstructionScript`)