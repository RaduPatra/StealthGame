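; Test AI controller for NPCs that exposes manual triggers and perception debugging.
; BeginPlay enables input from player controller 0 so the G key calls ActiveTurn, and detection state changes are relayed through StateChanged.
; A helper prints an actor's last sensed stimuli per sense class, but the debug chains using it are disconnected and the perception update event is empty.
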(event `self.AIPerception.OnTargetPerceptionUpdated`
  (params (Actor :type "Actor Object Reference") (Stimulus :type "AIStimulus Structure"))
  ;[1 0.2656 0.2656] Perception Debug
)

(event `Key|F`
  (params (Key :type "Key Structure"))
  ;[1 0.2656 0.2656] Perception Debug
)

(event `self.ReceivePossess`
  (params (PossessedPawn :type "Pawn Object Reference")))

(event `self.ReceiveBeginPlay`
  (`self.EnableInput` (`GameplayStatics.GetPlayerController` 0)))

(event `self.OnDetectionStateChange`
  (params (DetectionState :type "EDetectionState Enum" :default "Neutral"))
  (`self.StateChanged` DetectionState))

(event `Key|G` :consume false
  (params (Key :type "Key Structure"))
  ;[1 0.2656 0.2656] Perception Debug
  (:`Pressed`
    (`KismetSystemLibrary.PrintString` "G pressed")
    (`self.CallActiveTurn`)))

(event `Key|F`
  (params (Key :type "Key Structure"))
  ;[1 0.2656 0.2656] Perception Debug
)

(fn `GetPrecievedActorsStimuliInfo`
  (params (self2 :type "AIPerceptionComponent Object Reference") (Actor :type "Actor Object Reference"))
  (bind (_info _returnvalue) (`AIPerceptionComponent.GetActorsPerception` self2 Actor))
  (`KismetSystemLibrary.PrintString` (`KismetStringLibrary.Concat_StrStr` "sensed " (`KismetStringLibrary.Conv_BoolToString` _returnvalue) " \n"))
  (bind (_target _lastsensedstimuli) (break `ActorPerceptionBlueprintInfo` _info))
  (for _array_element _lastsensedstimuli
    (bind _returnvalue_2 (`AIPerceptionSystem.GetSenseClassForStimulus` _array_element))
    (`KismetSystemLibrary.PrintString` (`KismetStringLibrary.Concat_StrStr` "Sense Class:" (`KismetSystemLibrary.GetClassDisplayName` _returnvalue_2) " \n") true true (struct :`R` 0.116038 :`G` 1.0 :`B` 0.968162 :`A` 1.0))
    (bind (_age _expirationage _strength _stimuluslocation _receiverlocation _tag _bsuccessfullysensed) (break `AIStimulus` _array_element))
    (`KismetSystemLibrary.PrintString` (`KismetStringLibrary.Concat_StrStr` (`KismetStringLibrary.Conv_DoubleToString` _age) " \n" (`KismetStringLibrary.Conv_DoubleToString` _expirationage) " \n" (`KismetStringLibrary.Conv_DoubleToString` _strength) " \n" (`KismetStringLibrary.Conv_VectorToString` _receiverlocation) " \n" (`KismetStringLibrary.Conv_BoolToString` _bsuccessfullysensed) " \n" (`KismetSystemLibrary.GetDisplayName` _target) " \n"))))

(fn `UserConstructionScript`)