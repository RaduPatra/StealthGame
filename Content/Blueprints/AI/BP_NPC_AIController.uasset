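; AI controller for NPCs that reacts to suspicion detection states and the death of its pawn.
; Detection changes are passed on through CallStateChanged and set the NPC character's IsAttacking flag, true only in Alert.
; Health depletion stops the brain logic and suspicion detection, clears focus and disables sight and hearing.
; Target and perception events are empty, while the EQS chase-slot query and perception debug printing are left disconnected.
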(event `self.AIPerception.OnTargetPerceptionUpdated`
  (params (Actor :type "Actor Object Reference") (Stimulus :type "AIStimulus Structure"))
  ;[1 0.2656 0.2656] Perception Debug
)

(event `Key|F`
  (params (Key :type "Key Structure"))
  ;[1 0.2656 0.2656] Perception Debug
)

(event `Key|G` :consume false
  (params (Key :type "Key Structure"))
  ;[1 0.2656 0.2656] Perception Debug
)

(event `self.ReceiveBeginPlay`
  (add `SGHealthComponent.OnHealthDepleted` (`self.GetComponentByClass` (`self.K2_GetPawn`) "/Script/StealthGame.SGHealthComponent") (delegate `OnDeath`)))

(event `OnDeath`
  (params (DamageCauser :type "Actor Object Reference"))
  (`self.HandleDeath`))

(event `HandleDeath`
  (`BrainComponent.StopLogic` (`self.BrainComponent`) "Died")
  (`self.ToggleSuspicionDetection` false)
  (`self.K2_ClearFocus`)
  (`AIPerceptionComponent.SetSenseEnabled` (`self.AIPerception`) "/Script/AIModule.AISense_Hearing" false)
  (`AIPerceptionComponent.SetSenseEnabled` (`self.AIPerception`) "/Script/AIModule.AISense_Sight" false))

(event `self.OnDetectionStateChange`
  (params (DetectionState :type "EDetectionState Enum" :default "Neutral"))
  (`self.StateChanged` DetectionState)
  (bind _asbp_npc_character (cast `/Game/Blueprints/AI/BP_NPC_Character` (`self.ControlledPawn`)))
  (switch `EDetectionState` DetectionState
    (:`Neutral`
      (set `/Game/Blueprints/AI/BP_NPC_Character.Is Attacking` false _asbp_npc_character :!label _label))
    (:`Searching`
      (goto _label))
    (:`Investigating`
      (goto _label))
    (:`Alert`
      (set `/Game/Blueprints/AI/BP_NPC_Character.Is Attacking` true _asbp_npc_character))))

(event `self.OnTargetAcquired`
  (params (Target :type "Actor Object Reference")))

(event `OnQueryFinishedEvent_Event_0`
  (params (QueryInstance :type "EnvQueryInstanceBlueprintWrapper Object Reference") (QueryStatus :type "EEnvQueryStatus Enum" :default "Processing"))
  (bind _resultlocations (`EnvQueryInstanceBlueprintWrapper.GetQueryResultsAsLocations` QueryInstance))
  (if (> (`KismetArrayLibrary.Array_Length` _resultlocations) 0)
    (bind _slot (message `/Game/Blueprints/AI/Test/BPI_SlotAITargetTest.CreateTargetSlot` (stale `self.OnTargetAcquired` Target) (`|GetArrayItem` _resultlocations) self))
    (`BlackboardComponent.SetValueAsObject` (`self.Blackboard`) (`self.TargetChaseSlotKey`) _slot)
    (else
      (`KismetSystemLibrary.PrintString` "No Slot Location Available"))))

(event `self.OnTargetLost`
  (params (Target :type "Actor Object Reference")))

(fn `GetPrecievedActorsStimuliInfo`
  (params (self2 :type "AIPerceptionComponent Object Reference") (Actor :type "Actor Object Reference"))
  (bind (_info _returnvalue) (`AIPerceptionComponent.GetActorsPerception` self2 Actor))
  (`KismetSystemLibrary.PrintString` (`KismetStringLibrary.Concat_StrStr` "sensed " (`KismetStringLibrary.Conv_BoolToString` _returnvalue) " \n"))
  (bind (_target _lastsensedstimuli) (break `ActorPerceptionBlueprintInfo` _info))
  (for _array_element _lastsensedstimuli
    (bind _returnvalue_2 (`AIPerceptionSystem.GetSenseClassForStimulus` _array_element))
    (`KismetSystemLibrary.PrintString` (`KismetStringLibrary.Concat_StrStr` "Sense Class:" (`KismetSystemLibrary.GetClassDisplayName` _returnvalue_2) " \n") true true (struct :`R` 0.116038 :`G` 1.0 :`B` 0.968162 :`A` 1.0))
    (bind (_age _expirationage _strength _stimuluslocation _receiverlocation _tag _bsuccessfullysensed) (break `AIStimulus` _array_element))
    (`KismetSystemLibrary.PrintString` (`KismetStringLibrary.Concat_StrStr` (`KismetStringLibrary.Conv_DoubleToString` _age) " \n" (`KismetStringLibrary.Conv_DoubleToString` _expirationage) " \n" (`KismetStringLibrary.Conv_DoubleToString` _strength) " \n" (`KismetStringLibrary.Conv_VectorToString` _receiverlocation) " \n" (`KismetStringLibrary.Conv_BoolToString` _bsuccessfullysensed) " \n" (`KismetSystemLibrary.GetDisplayName` _target) " \n"))))

(fn `UserConstructionScript`)