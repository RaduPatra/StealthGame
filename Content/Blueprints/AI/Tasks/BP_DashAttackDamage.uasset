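; AI task that gives the controlled pawn's dash attack a damage collider aimed at the player team.
; SetupDamageCollision spawns a BP_DamageCollider at the pawn's location (the forward offset receives a zero vector) and attaches it to the pawn.
; When the collider damages a target, the task cancels the dash gameplay action and finishes as succeeded.
; TaskFinished destroys any remaining collider.
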(event Custom|OnDamagedTarget_Event
  (Class|SGameplayAction|CancelAction (Variables|Default|GetDashGameplayAction))
  (Class|SGBTTaskDashAttack|FinishTask "Succeeded"))

(event EventSetupDamageCollision
  (bind _returnvalue (CallFunction|GetControlledPawn))
  (bind _returnvalue_2 (Game|SpawnActorfromClass "/Game/Blueprints/AI/BP_DamageCollider.BP_DamageCollider_C" (Math|Conversions|ToTransform(Vector) (|(Loc+(Fwd*Scalar)) :Loc (Transformation|GetActorLocation (CallFunction|GetControlledPawn)) :Scalar 3e+02)) "AdjustIfPossibleButAlwaysSpawn" "MultiplyWithRoot" _returnvalue "(TagName=\"Character.Player\")" _returnvalue))
  (Variables|Default|SetSpawnedDamageCollider _returnvalue_2)
  (Transformation|AttachActorToActor (Variables|Default|GetSpawnedDamageCollider) (CallFunction|GetControlledPawn) "None" "KeepWorld" "KeepRelative" "KeepRelative" true)
  (EventDispatchers|AssignOnDamagedTarget (Variables|Default|GetSpawnedDamageCollider) (delegate Custom|OnDamagedTarget_Event)))

(event EventTaskFinished
  (params (TaskResult :type EBTNodeResult%20Enum :default "Succeeded"))
  (bind _spawneddamagecollider (Variables|Default|GetSpawnedDamageCollider))
  (Utilities|IsValid _spawneddamagecollider
    (:Is%20Valid
      (Actor|DestroyActor _spawneddamagecollider))))

(fn GetControlledPawn
  (return (Pawn|GetControlledPawn (AI|GetAIController (Components|GetOwner (Class|BTFunctionLibrary|GetOwnerComponent))))))

(fn IgnoreCollisions
  (params (DamageActor :type BP%20Damage%20Collider%20Object%20Reference))
  (CallFunction|IgnoreActorCollisions 0 (CallFunction|GetControlledPawn)))