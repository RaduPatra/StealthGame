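; BP_DamageCollider is an AI damage hitbox actor that deals a single hit on behalf of its owner.
; On BeginPlay it and its owner ignore each other's collisions.
; A box overlap reads the other actor's team tag and, on an exact match with TeamToDamage, applies BaseDamage with the owner as causer and instigator.
; A Damaged flag, never reset here, blocks further hits, and OnDamagedTarget is called after the hit.
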(event `self.ReceiveBeginPlay`
  (`/Game/Blueprints/BP_MyFunctionLibrary.IgnoreActorCollisions` self (`self.GetOwner`))
  (`/Game/Blueprints/BP_MyFunctionLibrary.IgnoreActorCollisions` (`self.GetOwner`) self))

(event `self.Box.OnComponentBeginOverlap`
  (params (OverlappedComponent :type "PrimitiveComponent Object Reference") (OtherActor :type "Actor Object Reference") (OtherComp :type "PrimitiveComponent Object Reference") (OtherBodyIndex :type Integer) (bFromSweep :type Boolean) (SweepResult :type "HitResult Structure (by ref)"))
  (bind _returnvalue (`self.GetOwner`))
  (bind _returnvalue_2 (message `SGCombatInterface.GetTeamTag` OtherActor))
  (if (and (not (`self.Damaged`)) (`BlueprintGameplayTagLibrary.MatchesTag` _returnvalue_2 (`self.TeamToDamage`) true))
    (`SGHealthComponent.ApplyDamageToActor` OtherActor (make `DamageInfo` _returnvalue _returnvalue (`self.Base Damage`)))
    (set `self.Damaged` true)
    (`self.OnDamagedTarget`)))

(fn `UserConstructionScript`)