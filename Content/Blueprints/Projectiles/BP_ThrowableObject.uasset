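; Throwable physics object projectile that reports noise once it comes to rest and can be picked up through its interaction component.
; When the box body goes to sleep, it disables physics and reports a noise event at its location, tagged with its interactable type.
; On interaction, it registers for the Action.Interacting tag event on the interactor's gameplay action component, then destroys itself when that callback fires.
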(event `self.ReceiveBeginPlay`
  (set `InteractionComponent.OnCanInteract` (`|CreateDelegate` :!event `CanInteract`) (`self.InteractionComponent`)))

(event `self.InteractionComponent.OnInteract`
  (params (Interactor :type "SInteractor Object Reference"))
  (`ISGTagEventInterface.RegisterGameplayTagEvent2` (`self.GetComponentByClass` (`ActorComponent.GetOwner` Interactor) "/Script/StealthGame.SGameplayActionComponent") (struct :`TagName` "Action.Interacting") (delegate `OnPickedUp`)))

(event `OnPickedUp`
  (`self.K2_DestroyActor`))

(event `self.BoxComponent.OnComponentSleep`
  (params (SleepingComponent :type "PrimitiveComponent Object Reference") (BoneName :type Name))
  ;[1 1 1] Report noise on land
  (set `self.IsBoxSleeping` true)
  (`PrimitiveComponent.SetSimulatePhysics` (`self.BoxComponent`) false)
  (`AISense_Hearing.ReportNoiseEvent` (`self.K2_GetActorLocation`) 1.0 self 0.0 (`BlueprintGameplayTagLibrary.GetTagName` (`InteractionComponent.InteractableType` (`self.InteractionComponent`)))))

(event `self.ReceiveActorBeginOverlap`
  (params (OtherActor :type "Actor Object Reference")))

(event `self.BoxComponent.OnComponentBeginOverlap`
  (params (OverlappedComponent :type "PrimitiveComponent Object Reference") (OtherActor :type "Actor Object Reference") (OtherComp :type "PrimitiveComponent Object Reference") (OtherBodyIndex :type Integer) (bFromSweep :type Boolean) (SweepResult :type "HitResult Structure (by ref)")))

(fn `GetLocation`
  (returns (Location :type "Vector Structure"))
  (return (`self.K2_GetActorLocation`)))

(fn `GetRotation`
  (returns (Rotation :type "Rotator Structure"))
  (return))

(fn `ThrowOld`
  (params (Velocity :type "Vector Structure")))

(fn `UserConstructionScript`)