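; Prototype base projectile that uses the SG object pooling subsystem, with Speed and GravityScale applied to its movement component at construction.
; Pooled begin and end play toggle ignoring the owner on the Box collider, resetting and activating or deactivating movement.
; A Box hit calls the projectile hit handler, spawns the impact particle and releases the actor to the pool.
; Lifetime timer logic is left unconnected, so only hits trigger release here.
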(event `self.ReceiveBeginPlay`)

(event `self.Box.OnComponentHit`
  (params (HitComponent :type "PrimitiveComponent Object Reference") (OtherActor :type "Actor Object Reference") (OtherComp :type "PrimitiveComponent Object Reference") (NormalImpulse :type "Vector Structure") (Hit :type "HitResult Structure (by ref)"))
  (`self.OnProjectileHit` OtherActor Hit)
  (`GameplayStatics.SpawnEmitterAtLocation` (`self.ImpactParticle`) (`.Location` (`GameplayStatics.BreakHitResult` Hit)) (struct) (1.0 1.0 1.0) true "AutoRelease")
  (bind _returnvalue (`SGObjectPoolingSubsystem.ReleaseActorToPool` (subsystem `SGObjectPoolingSubsystem`) self))
  (if (not _returnvalue)
    (`KismetSystemLibrary.PrintString` "failed to release")))

(event `self.PooledBeginPlay`
  (`PrimitiveComponent.IgnoreActorWhenMoving` (`self.Box`) (`self.GetOwner`) true)
  (`SGBlueprintFunctionLibrary.ResetMovementComp` (`self.ProjectileMovement`))
  (`ActorComponent.Activate` (`self.ProjectileMovement`) true))

(event `CustomEvent_0`
  (`SGObjectPoolingSubsystem.ReleaseActorToPool` (subsystem `SGObjectPoolingSubsystem`) self))

(event `self.PooledEndPlay`
  (`PrimitiveComponent.IgnoreActorWhenMoving` (`self.Box`) (`self.GetOwner`) false)
  (`ActorComponent.Deactivate` (`self.ProjectileMovement`)))

(fn `UserConstructionScript`
  (bind _projectilemovement (`self.ProjectileMovement`))
  (set `ProjectileMovementComponent.InitialSpeed` (`self.Speed`) _projectilemovement)
  (set `ProjectileMovementComponent.ProjectileGravityScale` (`self.GravityScale`) _projectilemovement))