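; Prototype fireball projectile Blueprint that works with object pooling and leaves its other behavior to its parent class.
; On pooled begin play it calls the parent, then activates its particle system with a reset; on pooled end play it deactivates it.
; Overlap and Tick are disabled, and stray Box and particle deactivation calls never run.
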(event `self.ReceiveBeginPlay`
  (`parent.ReceiveBeginPlay`))

(event `self.PooledEndPlay`
  (`parent.PooledEndPlay`)
  (`ActorComponent.Deactivate` (`self.ParticleSystem`)))

(event `self.PooledBeginPlay`
  (`parent.PooledBeginPlay`)
  (`ActorComponent.Activate` (`self.ParticleSystem`) true))

(fn `UserConstructionScript`
  (`parent.UserConstructionScript`))