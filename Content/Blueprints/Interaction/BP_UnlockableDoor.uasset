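; Interactable hinged door with Opened, Closed and Locked states that swings away from whoever opens it.
; A dot product against the frame picks the swing side for a timeline rotation, with collision off while moving and state changes broadcast on finish.
; When locked, the Interaction component grants an unlock gameplay action, gated by a key tag; uncancelled completion unlocks it.
; Getters supply a montage and side-dependent reference transforms.
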(event `self.RegisterStateChange`
  (params (OnOpenStateChanged :type "Delegate (by ref)"))
  (add `self.OnDoorStateChanged` OnOpenStateChanged))

(event `self.ReceiveBeginPlay`
  (set `InteractionComponent.OnCanInteract` (`|CreateDelegate` :!event `CanInteractNew`) (`self.Interaction`))
  (`self.SetInitialState`))

(event `self.Interaction.OnInteract`
  (params (Interactor :type "SInteractor Object Reference"))
  (switch `EOpenState` (`self.DoorState`)
    (:`Opened`
      (bind _sign (`self.Get Dot Side Sign` (`self.K2_GetActorLocation` (`ActorComponent.GetOwner` Interactor)) :!label _label)) ; always unlock door away from interactor
      (set `self.DotSign` _sign)
      (set `self.IsDoorMoving` true)
      (`PrimitiveComponent.SetCollisionEnabled` (`self.SM_Door`) "NoCollision") ; for now this will do, need to handle physics properly in the future
      (switch `EOpenState` (`self.DoorState`)
        (:`Opened`
          (set `self.DotSignToUse` (`self.PreviousOpenSign`))
          (bind (_direction _dooropen) (`Timeline|DoorTimeline` :!via `ReverseFromEnd` :!label _label_2)
            (:`Update`
              (`SceneComponent.K2_SetRelativeRotation` (`self.SM_Door`) (`KismetMathLibrary.MakeRotator` 0.0 0.0 (* _dooropen (`self.DotSignToUse`))) false false))
            (:`Finished`
              (`self.FinishMovingDoor` _direction))))
        (:`Closed`
          (set `self.DotSignToUse` (`self.DotSign`))
          (goto _label_2 :!via `PlayFromStart`))))
    (:`Closed`
      (goto _label))
    (:`Locked`
      (if true
        _))))

(event `self.ReceiveTick`
  (params (DeltaSeconds :type "Float (single-precision)")))

(event `self.Interaction.OnInteractFinished`
  (params (Interactor :type "SInteractor Object Reference") (bCancelled :type Boolean))
  (`self.ChangeInteractionDataForState` (`self.DoorState`) bCancelled))

(fn `Can Interact`
  (params (Interactor :type "SInteractor Object Reference"))
  (returns (ReturnValue :type Boolean))
  (return (or (and (`BlueprintGameplayTagLibrary.HasTag` (`SGameplayActionComponent.OtherTags` (`self.GetComponentByClass` (`ActorComponent.GetOwner` Interactor) "/Script/StealthGame.SGameplayActionComponent")) (`self.KeyTag`) true) (`|EnumEquality` (`self.DoorState`) "Locked")) (and (`|EnumInequality` (`self.DoorState`) "Locked") (not (`self.IsDoorMoving`))))))

(fn `Can InteractOld`
  (returns (ReturnValue :type Boolean))
  (`KismetSystemLibrary.PrintString` "CanINteract")
  (return (not (`self.IsDoorMoving`))))

(fn `CanInteractNew`
  (params (Interactor :type "SInteractor Object Reference"))
  (returns (ReturnValue :type "InteractResult Structure"))
  (if (and (not (`self.DoesInteractorHaveKey` Interactor)) (`|EnumEquality` (`self.DoorState`) "Locked"))
    (return (make `InteractResult` false (struct :`TagName` "Actor.Interactable.FailReason.MissingKey")))
    (elif (`self.IsDoorMoving`)
      (return (make `InteractResult` false))
      (else
        (return (make `InteractResult` true (struct :`TagName` "Actor.Interactable.FailReason.MissingKey")))))))

(fn `ChangeInteractionDataForState`
  (params (DoorState :type "EOpenState Enum" :default "Opened") (InteractionCancelled :type Boolean))
  (switch `EOpenState` DoorState
    (:`Opened`
      (set `self.DoorInteractionText` "Open Door")
      (`InteractionComponent.ChangeInteractionData` (`self.Interaction`) (make `InteractionData` "/Game/Blueprints/Abilities/GA_EmptyAction.GA_EmptyAction_C" (`self.DoorInteractionText`)) :!label _label))
    (:`Closed`
      (set `self.DoorInteractionText` "Close Door")
      (goto _label))
    (:`Locked`
      (if (not InteractionCancelled)
        (set `self.DoorState` "Closed")
        (set `self.DoorInteractionText` "Open  Door")
        (goto _label)))))

(fn `DoesInteractorHaveKey`
  (params (self2 :type "ActorComponent Object Reference"))
  (returns (ReturnValue :type Boolean))
  (return (`BlueprintGameplayTagLibrary.HasTag` (`SGameplayActionComponent.OtherTags` (`self.GetComponentByClass` (`ActorComponent.GetOwner` self2) "/Script/StealthGame.SGameplayActionComponent")) (`self.KeyTag`) true)))

(fn `FinishMovingDoor`
  (params (Direction :type "ETimelineDirection Enum" :default "Forward"))
  (set `self.IsDoorMoving` false)
  (`PrimitiveComponent.SetCollisionEnabled` (`self.SM_Door`) "QueryAndPhysics")
  (switch `ETimelineDirection` Direction
    (:`Forward`
      (set `self.DoorState` "Opened")
      (set `self.PreviousOpenSign` (`self.DotSign`)))
    (:`Backward`
      (set `self.DoorState` "Closed")))
  (`self.OnDoorStateChanged` (`self.DoorState`)))

(fn `Get Dot Side Sign`
  (params (InteractorLocation :type "Vector Structure"))
  (returns (Sign :type "Float (double-precision)"))
  (bind (_returnvalue_x _returnvalue_y) (`KismetMathLibrary.BreakVector` (`SceneComponent.GetForwardVector` (`self.SM_DoorFrame`))))
  (bind (_returnvalue_x_2 _returnvalue_y_2) (`KismetMathLibrary.BreakVector` (`KismetMathLibrary.GetDirectionUnitVector` InteractorLocation (`SceneComponent.K2_GetComponentLocation` (`self.SM_DoorFrame`)))))
  (return (`KismetMathLibrary.SignOfFloat` (`KismetMathLibrary.Dot_VectorVector` (`KismetMathLibrary.Normal` (`KismetMathLibrary.MakeVector` _returnvalue_x _returnvalue_y)) (`KismetMathLibrary.Normal` (`KismetMathLibrary.MakeVector` _returnvalue_x_2 _returnvalue_y_2))))))

(fn `GetLocation`
  (returns (Location :type "Vector Structure"))
  (locals (RefLocation :type "Vector Structure" :default (0.0 0.0 0.0)))
  (bind _sign (`self.Get Dot Side Sign` (`self.K2_GetActorLocation` (`ActorComponent.GetOwner` (`InteractionComponent.CurrentInteractor` (`self.Interaction`))))))
  (if (> _sign 0.0)
    (set `local.RefLocation` (`SceneComponent.K2_GetComponentLocation` (`self.RefSkeletalMeshFront`)))
    (else
      (set `local.RefLocation` (`SceneComponent.K2_GetComponentLocation` (`self.RefSkeletalMeshBack`)))))
  (return (`local.RefLocation`)))

(fn `GetOpenMontage`
  (returns (ReturnValue :type "AnimMontage Object Reference"))
  (locals (OpenMontage :type "AnimMontage Object Reference" :default "/Script/Engine.AnimMontage'/Game/Animations/Activate_Wall_KeyTurn_MidHeight_Montage.Activate_Wall_KeyTurn_MidHeight_Montage'"))
  (return (`self.Montage to Play`)))

(fn `GetOpenState`
  (returns (ReturnValue :type "EOpenState Enum"))
  (return (`self.DoorState`)))

(fn `GetRotation`
  (returns (Rotation :type "Rotator Structure"))
  (locals (RefLocation :type "Rotator Structure" :default (struct)))
  (bind _sign (`self.Get Dot Side Sign` (`self.K2_GetActorLocation` (`ActorComponent.GetOwner` (`InteractionComponent.CurrentInteractor` (`self.Interaction`))))))
  (if (> _sign 0.0)
    (set `local.RefLocation` (`KismetMathLibrary.Conv_VectorToRotator` (`SceneComponent.GetRightVector` (`self.RefSkeletalMeshFront`))))
    (else
      (set `local.RefLocation` (`KismetMathLibrary.Conv_VectorToRotator` (`SceneComponent.GetRightVector` (`self.RefSkeletalMeshBack`))))))
  (return (`local.RefLocation`)))

(fn `SetInitialState`
  (switch `EOpenState` (`self.DoorState`)
    (:`Opened`
      (`|ExecutionSequence` :!label _label
        (:`then_0`
          (if (`|EnumEquality` (`self.DoorState`) "Opened")
            (`SceneComponent.K2_SetRelativeRotation` (`self.SM_Door`) (`KismetMathLibrary.MakeRotator` 0.0 0.0 80.0) false false)
            (set `self.DoorInteractionText` "Close Door")))
        (:`then_1`
          (`InteractionComponent.ChangeInteractionData` (`self.Interaction`) (make `InteractionData` "/Game/Blueprints/Abilities/GA_EmptyAction.GA_EmptyAction_C" (`self.DoorInteractionText`))))))
    (:`Closed`
      (set `self.DoorInteractionText` "Open Door")
      (goto _label))
    (:`Locked`
      (`InteractionComponent.ChangeInteractionData` (`self.Interaction`) (make `InteractionData` (`self.UnlockDoorGameplayAction`) "Unlock Door")))))

(fn `UserConstructionScript`)