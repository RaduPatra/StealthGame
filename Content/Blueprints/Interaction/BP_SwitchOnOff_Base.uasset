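; Base interactable on/off lever switch that toggles an Opened/Closed state and broadcasts it to registered listeners, starting with the initial state on BeginPlay.
; Interacting plays a state-dependent lever montage, whose notifies mark the half-pull and flip the state on full pull.
; Cancelling before the half-pull reverses the montage from its current position.
; Getters supply the matching character montage and alignment transform, and a camera transition component is initialized.
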(event `self.ReceiveBeginPlay`
  ;[1 1 1] Setup
  (set `InteractionComponent.OnCanInteract` (`|CreateDelegate` :!event `CanInteractNew`) (`self.Interaction`))
  (bind _asabp_slide_lever (cast `/Game/Simple_Activations/Props/Wall_Slide_Lever/Animations/ABP_SlideLever` (`SkeletalMeshComponent.GetAnimInstance` (`self.Switch_Object_SkelMesh`))))
  (`|ExecutionSequence`
    (:`then_0`
      (switch `EOpenState` (`self.OpenState`)
        (:`Closed`
          (`/Game/Simple_Activations/Props/Wall_Slide_Lever/Animations/ABP_SlideLever.PullDown` _asabp_slide_lever) ; sets anim time to last frame
        )))
    (:`then_1`
      (`self.OnDoorStateChanged` (`self.OpenState`))
      (`/Game/Blueprints/Interaction/BP_InteractionCameraTransition.Initialize` (`self.BP_InteractionCameraTransition`) (`ChildActorComponent.ChildActor` (`self.RightCamActor`)) (`ChildActorComponent.ChildActor` (`self.RightCamActor`))))))

(event `self.Interaction.OnInteract`
  (params (Interactor :type "SInteractor Object Reference"))
  (`self.PullSwitch` (`ActorComponent.GetOwner` Interactor)))

(event `PullSwitch`
  (params (Instigator :type "Actor Object Reference"))
  (set `self.SwitchPulled` false)
  (set `self.SwitchHalfPulled` false)
  (`self.DecideSwitchMontage`)
  (bind _notifyname (`|PlayMontage` (`self.Switch_Object_SkelMesh`) (`self.Montage to Play`))
    (:`OnNotifyBegin`
      (switch `string` (`KismetStringLibrary.Conv_NameToString` _notifyname)
        (:`SwitchPulled`
          (set `self.SwitchPulled` true)
          (switch `EOpenState` (`self.OpenState`)
            (:`Opened`
              (set `self.OpenState` "Closed"))
            (:`Closed`
              (set `self.OpenState` "Opened")))
          (`self.OnDoorStateChanged` (`self.OpenState`) Instigator))
        (:`SwitchHalfPulled`
          (set `self.SwitchHalfPulled` true))))))

(event `self.Interaction.OnInteractFinished`
  (params (Interactor :type "SInteractor Object Reference") (bCancelled :type Boolean))
  (`|ExecutionSequence`
    (:`then_0`
      (if (and bCancelled (not (`self.SwitchHalfPulled`)))
        (bind _notifyname (`|PlayMontage` (`self.Switch_Object_SkelMesh`) (`self.Montage to Play`) -1.0 (`AnimInstance.Montage_GetPosition` (`SkeletalMeshComponent.GetAnimInstance` (`self.Switch_Object_SkelMesh`)) (`self.Montage to Play`)))
          (:`OnNotifyBegin`
            (if (== _notifyname "SwitchBegin")
              (set `self.SwitchPulled` true))))))))

(event `self.RegisterStateChange`
  (params (OnOpenStateChanged :type "Delegate (by ref)"))
  (add `self.OnDoorStateChanged` OnOpenStateChanged))

(fn `Can Interact`
  (params (Interactor :type "SInteractor Object Reference"))
  (returns (ReturnValue :type Boolean))
  (return (and (not (`self.IsInteracting`)) (`self.SwitchPulled`))))

(fn `CanInteractNew`
  (params (Interactor :type "SInteractor Object Reference"))
  (returns (ReturnValue :type "InteractResult Structure"))
  (if (`self.SwitchPulled`)
    (return (make `InteractResult` true))
    (else
      (return (make `InteractResult` false)))))

(fn `DecideSwitchMontage`
  (switch `EOpenState` (`self.OpenState`)
    (:`Opened`
      (set `self.Montage to Play` (`self.ObjectCloseAnimation`)))
    (:`Closed`
      (set `self.Montage to Play` (`self.ObjectOpenAnimation`)))))

(fn `GetLocation`
  (returns (Location :type "Vector Structure"))
  (return (`SceneComponent.K2_GetComponentLocation` (`self.RefSkeletalMesh`))))

(fn `GetOpenMontage`
  (returns (ReturnValue :type "AnimMontage Object Reference"))
  (locals (OpenMontage :type "AnimMontage Object Reference"))
  (switch `EOpenState` (`self.OpenState`)
    (:`Opened`
      (set `local.OpenMontage` (`self.CharacterCloseAnimation`)))
    (:`Closed`
      (set `local.OpenMontage` (`self.CharacterOpenAnimation`))))
  (return (`local.OpenMontage`)))

(fn `GetOpenState`
  (returns (ReturnValue :type "EOpenState Enum"))
  (return (`self.OpenState`)))

(fn `GetRotation`
  (returns (Rotation :type "Rotator Structure"))
  (return (`KismetMathLibrary.Conv_VectorToRotator` (`SceneComponent.GetRightVector` (`self.RefSkeletalMesh`)))))

(fn `UserConstructionScript`)