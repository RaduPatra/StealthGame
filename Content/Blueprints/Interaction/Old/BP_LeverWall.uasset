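; Interactable wall lever that toggles between Opened and Closed and broadcasts the change as a door state.
; On interact it plays the open or close montage on its skeletal mesh, flipping the state when the montage notify begins.
; At BeginPlay it binds the interaction component's can-interact check and pulls the slide lever AnimBP down if closed.
; Getters expose the state, matching character montage, and reference mesh location and facing.
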(event `self.ReceiveBeginPlay`
  (set `InteractionComponent.OnCanInteract` (`|CreateDelegate` :!event `Can Interact New`) (`self.Interaction`))
  (bind _asabp_slide_lever (cast `/Game/Simple_Activations/Props/Wall_Slide_Lever/Animations/ABP_SlideLever` (`SkeletalMeshComponent.GetAnimInstance` (`self.Wall_Slide_Lever_SkelMesh`))))
  (switch `EOpenState` (`self.OpenState`)
    (:`Closed`
      (`/Game/Simple_Activations/Props/Wall_Slide_Lever/Animations/ABP_SlideLever.PullDown` _asabp_slide_lever))))

(event `self.Interaction.OnInteract`
  (params (Interactor :type "SInteractor Object Reference"))
  (`KismetSystemLibrary.PrintString` "Interact")
  (`self.UseLever`))

(event `UseLever`
  (switch `EOpenState` (`self.OpenState`)
    (:`Opened`
      (set `self.Montage to Play` (`self.ObjectCloseAnimation`)))
    (:`Closed`
      (set `self.Montage to Play` (`self.ObjectOpenAnimation`))))
  (`|PlayMontage` (`self.Wall_Slide_Lever_SkelMesh`) (`self.Montage to Play`)
    (:`OnNotifyBegin`
      (switch `EOpenState` (`self.OpenState`)
        (:`Opened`
          (set `self.OpenState` "Closed"))
        (:`Closed`
          (set `self.OpenState` "Opened")))
      (`self.OnDoorStateChanged` (`self.OpenState`)))))

(event `self.RegisterStateChange`
  (params (OnOpenStateChanged :type "Delegate (by ref)")))

(fn `Can Interact`
  (returns (ReturnValue :type Boolean))
  (`KismetSystemLibrary.PrintString` "CanINteract")
  (return (not (`self.IsInteracting`))))

(fn `Can Interact New`
  (params (Interactor :type "SInteractor Object Reference"))
  (returns (ReturnValue :type Boolean))
  (return (not (`self.IsInteracting`))))

(fn `GetLocation`
  (returns (Location :type "Vector Structure"))
  (return (`SceneComponent.K2_GetComponentLocation` (`self.RefSkeletalMesh`))))

(fn `GetOpenMontage`
  (returns (ReturnValue :type "AnimMontage Object Reference"))
  (locals (OpenMontage :type "AnimMontage Object Reference"))
  (switch `EOpenState` (`self.OpenState`)
    (:`Opened`
      (set `local.OpenMontage` (`self.CharacterCloseAnimation`)))
    (:`Closed`
      (set `local.OpenMontage` (`self.CharacterOpenAnimation`))))
  (return (`local.OpenMontage`)))

(fn `GetOpenState`
  (returns (ReturnValue :type "EOpenState Enum"))
  (return (`self.OpenState`)))

(fn `GetRotation`
  (returns (Rotation :type "Rotator Structure"))
  (return (`KismetMathLibrary.Conv_VectorToRotator` (`SceneComponent.GetRightVector` (`self.RefSkeletalMesh`)))))

(fn `UserConstructionScript`)