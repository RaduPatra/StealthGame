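; BP_FallingThing is a light-bearing prop that drops when its linked Openable reports Opened, damaging actors it overlaps.
; An Openable state message turns on mesh physics and records the instigator, whose controller is credited for damage if it is a pawn.
; A Box1 overlap switches off the light, then after a short delay disables damage and sets the mesh to overlap pawns.
; The construction script applies the configurable light settings.
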(event `self.ReceiveBeginPlay`
  (bind _openable (`self.Openable`))
  (message `SOpenable.RegisterStateChange` _openable (delegate `OnSwitchStateChanged`))
  (bind _returnvalue (message `SOpenable.GetOpenState` _openable))
  (`self.OnSwitchStateChanged` _returnvalue))

(event `OnSwitchStateChanged`
  (params (OpenState :type "EOpenState Enum" :default "Opened") (Instigator :type "Actor Object Reference"))
  (set `self.FallCauser` Instigator)
  (switch `EOpenState` OpenState
    (:`Opened`
      (`PrimitiveComponent.SetSimulatePhysics` (`self.StaticMesh2`) true))))

(event `self.ReceiveActorBeginOverlap`
  (params (OtherActor :type "Actor Object Reference"))
  (if (`self.DamageEnabled`)
    (bind _damageinstigator (`self.Try Get Damage Instigator` (`self.FallCauser`)))
    (`SGHealthComponent.ApplyDamageToActor` OtherActor (make `DamageInfo` self _damageinstigator (`self.FallDamage`)))))

(event `self.StaticMesh2.OnComponentBeginOverlap`
  (params (OverlappedComponent :type "PrimitiveComponent Object Reference") (OtherActor :type "Actor Object Reference") (OtherComp :type "PrimitiveComponent Object Reference") (OtherBodyIndex :type Integer) (bFromSweep :type Boolean) (SweepResult :type "HitResult Structure (by ref)")))

(event `self.Box1.OnComponentBeginOverlap`
  (params (OverlappedComponent :type "PrimitiveComponent Object Reference") (OtherActor :type "Actor Object Reference") (OtherComp :type "PrimitiveComponent Object Reference") (OtherBodyIndex :type Integer) (bFromSweep :type Boolean) (SweepResult :type "HitResult Structure (by ref)"))
  (`LightComponent.SetIntensity` (`self.PointLight`) 0.0)
  (`KismetSystemLibrary.Delay` 1.0)
  (set `self.DamageEnabled` false)
  (`PrimitiveComponent.SetCollisionResponseToChannel` (`self.StaticMesh2`) "ECC_Pawn" "ECR_Overlap"))

(event `self.StaticMesh2.OnComponentHit`
  (params (HitComponent :type "PrimitiveComponent Object Reference") (OtherActor :type "Actor Object Reference") (OtherComp :type "PrimitiveComponent Object Reference") (NormalImpulse :type "Vector Structure") (Hit :type "HitResult Structure (by ref)")))

(fn `GetOpenMontage`
  (returns (Montage :type "AnimMontage Object Reference"))
  (return null))

(fn `GetOpenState`
  (returns (NewParam :type "/Game/Blueprints/Interaction/OpenStateEnum2 Enum"))
  (return "NewEnumerator0"))

(fn `NewFunction_0`
  (params (NewParam1 :type "AINoiseEvent Structure"))
  (returns (NewParam :type "AINoiseEvent Structure"))
  (return))

(fn `Try Get Damage Instigator`
  (params (FallCauserActor :type "Actor Object Reference"))
  (returns (DamageInstigator :type "Controller Object Reference"))
  (bind _fallcauser (`self.FallCauser`)
    (:`then`
      (bind _aspawn (cast `Pawn` _fallcauser)
        (:`then`
          (return (`Pawn.GetController` _aspawn)))
        (:`CastFailed`
          _)))
    (:`else`
      _))
  (return null))

(fn `UserConstructionScript`
  (bind _pointlight (`self.PointLight`))
  (`LightComponent.SetIntensity` _pointlight (`self.Brightness`))
  (`LightComponent.SetLightColor` _pointlight (`self.Color`) true)
  (`PointLightComponent.SetSourceRadius` _pointlight (`self.Source Radius`)))