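; Interaction camera transition that blends the player's view to a supplied camera while they interact with the owning actor.
; When active at BeginPlay, it binds to the owner's InteractionComponent start and finish events.
; On interact it blends to the right camera and disables character input; on finish, cancelled or not, it blends back and re-enables input.
; Initialize supplies both cameras, though the left one is never used here.
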(event `self.ReceiveBeginPlay`
  (bind _returnvalue (`Actor.GetComponentByClass` (`self.GetOwner`) "/Script/StealthGame.InteractionComponent"))
  (if (`self.IsTransitionActive`)
    (add `InteractionComponent.OnInteract` _returnvalue (delegate `OnInteract`))
    (add `InteractionComponent.OnInteractFinished` _returnvalue (delegate `OnInteractFinished`))))

(event `OnInteractFinished`
  (params (Interactor :type "SInteractor Object Reference") (bCancelled :type Boolean))
  (`self.HandleInteractFinished` Interactor bCancelled))

(event `OnInteract`
  (params (Interactor :type "SInteractor Object Reference"))
  (`self.HandleOnInteract` Interactor))

(event `HandleOnInteract`
  (params (Interactor :type "SInteractor Object Reference"))
  (bind (_ascharacter _asplayer_controller) (`self.TryGetPlayerInfo` Interactor)
    (:`then`
      (`PlayerController.SetViewTargetWithBlend` _asplayer_controller (`self.RightTransitionCam`) 1.0 "VTBlend_Linear" 0.0 false)
      (`Actor.DisableInput` _ascharacter _asplayer_controller))))

(event `HandleInteractFinished`
  (params (Interactor :type "SInteractor Object Reference") (bCancelled :type Boolean))
  (bind (_ascharacter _asplayer_controller) (`self.TryGetPlayerInfo` Interactor)
    (:`then`
      (`PlayerController.SetViewTargetWithBlend` _asplayer_controller _ascharacter 0.5 "VTBlend_Linear" 0.0 false)
      (`Actor.EnableInput` _ascharacter _asplayer_controller))))

(fn `Initialize`
  (params (RightCam :type "Actor Object Reference") (LeftCam :type "Actor Object Reference"))
  (set `self.RightTransitionCam` RightCam)
  (set `self.LeftTransitionCam` LeftCam))