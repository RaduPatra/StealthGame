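; Charge-then-burst fireball ability that can only start while the owner is moving on the ground.
; A montage drives it: the charge notify waits, jumps to the charge-end section and sends a ChargeFinish event, while shoot notifies fire projectiles.
; Play rate scales to the shot delay until the projectile cap triggers the fire-end section.
; Projectiles come from an object pool, aimed from a socket at the owner's target location.
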(event `self.ReceiveActionActivated`
  (bind _mesh (`Character.Mesh` (`self.OwnerCharacter`)))
  (bind _ascharacter (cast `Character` (`self.OwnerActor`))
    (:`then`
      (set `self.OwnerCharacter` _ascharacter)
      (set `self.ShootLoopPlayRate` (/ 1.0 (`self.ShootDelay`)))
      (bind _notifyname (`|PlayMontage` _mesh "/Game/Animations/Fireball_1__UE_Montage.Fireball_1__UE_Montage")
        (:`then`
          (set `self.ProjectileSpawnCount` 0))
        (:`OnCompleted`
          (`self.FinishAction` :!label _label))
        (:`OnInterrupted`
          (goto _label))
        (:`OnNotifyBegin`
          (switch `string` (`KismetStringLibrary.Conv_NameToString` _notifyname)
            (:`Shoot`
              (`self.ShootProjectile`))
            (:`StartCharge`
              (`KismetSystemLibrary.Delay` (`self.CharageDuration`))
              (`AnimInstance.Montage_JumpToSection` (`SkeletalMeshComponent.GetAnimInstance` _mesh) (`self.ChargeEndSectionName`) "/Game/Animations/Fireball_1__UE_Montage.Fireball_1__UE_Montage")
              (`ISGTagEventInterface.SendGameplayEvent2` (`self.OwnerComponent`) (struct :`TagName` "Action.Event.ChargeFinish")))))))
    (:`CastFailed`
      (`self.CancelAction`))))

(event `ShootProjectile`
  (`AnimInstance.Montage_SetPlayRate` (`SkeletalMeshComponent.GetAnimInstance` (`Character.Mesh` (`self.OwnerCharacter`))) (`Character.GetCurrentMontage` (`self.OwnerCharacter`)) (`self.ShootLoopPlayRate`))
  (`self.SpawnProjectile`)
  (`/Engine/EditorBlueprintResources/StandardMacros.IncrementInt` (`self.ProjectileSpawnCount`)
    (:`  `
      (if (not (< (`self.ProjectileSpawnCount`) (`self.MaxProjectileSpawn`)))
        (`AnimInstance.Montage_JumpToSection` (`SkeletalMeshComponent.GetAnimInstance` (`Character.Mesh` (`self.OwnerCharacter`))) (`self.FireEndSectionName`) "/Game/Animations/Fireball_1__UE_Montage.Fireball_1__UE_Montage")
        (`AnimInstance.Montage_SetPlayRate` (`SkeletalMeshComponent.GetAnimInstance` (`Character.Mesh` (`self.OwnerCharacter`))) (`Character.GetCurrentMontage` (`self.OwnerCharacter`)) 1.0)))))

(event `self.ReceiveActionEnded`
  (bind _returnvalue (`SkeletalMeshComponent.GetAnimInstance` (`Character.Mesh` (`self.OwnerCharacter`))))
  (if (`AnimInstance.Montage_IsActive` _returnvalue "/Game/Animations/Fireball_1__UE_Montage.Fireball_1__UE_Montage")
    (`AnimInstance.Montage_Stop` _returnvalue 0.2 "/Game/Animations/Fireball_1__UE_Montage.Fireball_1__UE_Montage")))

(event `self.ReceiveTickAction`
  (params (DeltaTime :type "Float (single-precision)")))

(fn `ReceiveCanStart`
  (params (NewActionData :type "GameplayActionData Structure (by ref)") (OwnerComp :type "SGameplayActionComponent Object Reference"))
  (returns (ReturnValue :type Boolean))
  (return (`NavMovementComponent.IsMovingOnGround` (`Actor.GetComponentByClass` (`self.OwnerActor`) "/Script/Engine.CharacterMovementComponent"))))

(fn `SpawnProjectile`
  (bind _ownercharacter (`self.OwnerCharacter`))
  (bind _returnvalue (`SceneComponent.GetSocketLocation` (`Character.Mesh` (`self.OwnerCharacter`)) (`self.ShootSocketName`)))
  (bind _location (message `/Game/Blueprints/Player/BPI_Shooter.Get Shoot Target Location` (`self.OwnerCharacter`)))
  (bind _returnvalue_2 (`SGObjectPoolingSubsystem.GetActorFromPool` (subsystem `SGObjectPoolingSubsystem`) (`self.ProjectileClass`) (`KismetMathLibrary.MakeTransform` _returnvalue (`KismetMathLibrary.FindLookAtRotation` _returnvalue _location)) _ownercharacter _ownercharacter))
  (`PrimitiveComponent.IgnoreActorWhenMoving` (`Character.CapsuleComponent` _ownercharacter) _returnvalue_2 true))