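; Throw action that turns the owner to its aim rotation and plays a robot police grenade-throw montage to launch a projectile.
; It can start only while moving on ground, and sets the throw velocity before an async turn through the owner's TurnInPlace component.
; The montage follows the turn, with its notify triggering the throw and completion or interruption finishing the action.
; Ending the action interrupts the turn.
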(event `self.ReceiveActionActivated`
  (bind _returnvalue (`Actor.GetComponentByClass` (`ActorComponent.GetOwner` (`self.OwnerComponent`)) "/Script/StealthGame.TurnInPlaceComponent"))
  (`/Engine/EditorBlueprintResources/StandardMacros.IsValid` _returnvalue
    (:`Is Valid`
      (`self.SetThrowVelocity`)
      (`AsyncTurnInPlace.AsyncTurnInPlace` _returnvalue (`Pawn.GetBaseAimRotation` (`PawnMovementComponent.GetPawnOwner` (`self.CharacterMovementComponent`)))
        (:`OnCompleted`
          (`self.OnTurnFinished_Event`))))
    (:`Is Not Valid`
      (`KismetSystemLibrary.PrintString` "GA_Throw: Owner MIssing TurnInPlace Comp"))))

(event `OnTurnFinished_Event`
  (`|PlayMontage` (`Character.Mesh` (`CharacterMovementComponent.GetCharacterOwner` (`self.CharacterMovementComponent`))) "/Game/Animations/RobotPolice_GrenadeThrow_Montage.RobotPolice_GrenadeThrow_Montage" 1.1 0.1
    (:`OnCompleted`
      (`self.FinishAction` :!label _label))
    (:`OnInterrupted`
      (goto _label))
    (:`OnNotifyBegin`
      (`self.ThrowProjectile`))))

(event `self.ReceiveActionEnded`
  (`TurnInPlaceComponent.InterruptTurnInPlace` (`Actor.GetComponentByClass` (`ActorComponent.GetOwner` (`self.OwnerComponent`)) "/Script/StealthGame.TurnInPlaceComponent")))

(fn `ReceiveCanStart`
  (params (NewActionData :type "GameplayActionData Structure (by ref)") (OwnerComp :type "SGameplayActionComponent Object Reference"))
  (returns (ReturnValue :type Boolean))
  (return (`NavMovementComponent.IsMovingOnGround` (`Actor.GetComponentByClass` (`ActorComponent.GetOwner` OwnerComp) "/Script/Engine.CharacterMovementComponent"))))