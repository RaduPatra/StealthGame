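; Interaction ability that plays an openable object's montage on the owning Character, motion-warped to the object.
; It can start only if the Instigator implements SOpenable and a short horizontal capsule trace from the owner hits it on the expected object channel.
; The Instigator supplies montage, location and rotation; the "LeverWarp" target is set just after playback starts.
; Montage completion or interruption finishes the action, and ending it stops the montage.
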(event `self.ReceiveActionActivated`
  (bind _instigator (`self.Instigator`))
  (bind _ascharacter (cast `Character` (`self.OwnerActor`))
    (:`then`
      (bind _returnvalue (message `SOpenable.GetOpenMontage` (`self.Instigator`)))
      (`|PlayMontage` (`Character.Mesh` _ascharacter) _returnvalue
        (:`then`
          (bind _location (message `/Game/Blueprints/Interaction/IInteractablePositionProvider.GetLocation` _instigator))
          (bind _rotation (message `/Game/Blueprints/Interaction/IInteractablePositionProvider.GetRotation` _instigator))
          (`MotionWarpingComponent.AddOrUpdateWarpTargetFromLocationAndRotation` (`Actor.GetComponentByClass` (`self.OwnerActor`) "/Script/MotionWarping.MotionWarpingComponent") "LeverWarp" _location _rotation))
        (:`OnCompleted`
          (`self.FinishAction`))
        (:`OnInterrupted`
          (`self.FinishAction`))))
    (:`CastFailed`
      (`self.CancelAction`))))

(event `self.ReceiveActionEnded`
  (bind _returnvalue (message `SOpenable.GetOpenMontage` (`self.Instigator`)))
  (`Character.StopAnimMontage` (cast `Character` (`self.OwnerActor`) :!pure true) _returnvalue))

(fn `ReceiveCanStart`
  (params (NewActionData :type "GameplayActionData Structure (by ref)") (OwnerComp :type "SGameplayActionComponent Object Reference"))
  (returns (ReturnValue :type Boolean))
  (locals (ObjectTypes :type "Array of EObjectTypeQuery Enum") (InstigatorActor :type "Actor Object Reference") (ActionOwner :type "Actor Object Reference"))
  (bind _returnvalue (`Actor.GetComponentByClass` (`local.ActionOwner`) "/Script/Engine.CapsuleComponent"))
  (bind _returnvalue_2 (`Actor.K2_GetActorLocation` (`local.ActionOwner`)))
  (bind (_returnvalue_x _returnvalue_y) (`KismetMathLibrary.BreakVector` (`KismetMathLibrary.GetDirectionUnitVector` _returnvalue_2 (`Actor.K2_GetActorLocation` (`local.InstigatorActor`)))))
  (if (`KismetSystemLibrary.DoesImplementInterface` (`self.Instigator`) "/Script/StealthGame.SOpenable")
    (set `local.InstigatorActor` (`.Instigator` (break `GameplayActionData` NewActionData)))
    (set `local.ActionOwner` (`ActorComponent.GetOwner` OwnerComp))
    (bind _outhit (`KismetSystemLibrary.CapsuleTraceSingleForObjects` _returnvalue_2 (+ _returnvalue_2 (* (`KismetMathLibrary.MakeVector` _returnvalue_x _returnvalue_y) 200.0)) (`CapsuleComponent.CapsuleRadius` _returnvalue) (`CapsuleComponent.CapsuleHalfHeight` _returnvalue) (`|MakeArray` "ObjectTypeQuery7" "ObjectTypeQuery1" "ObjectTypeQuery5" "ObjectTypeQuery4" "ObjectTypeQuery2" :!type "EObjectTypeQuery Enum") false (`|MakeArray` (`local.ActionOwner`)) "ForDuration" true (struct :`R` 1.0 :`A` 1.0) (struct :`G` 1.0 :`A` 1.0) 0.4))
    (bind (_bblockinghit _binitialoverlap _time _distance _location _impactpoint _normal _impactnormal _physmat _hitactor _hitcomponent) (`GameplayStatics.BreakHitResult` _outhit))
    (`/Engine/EditorBlueprintResources/StandardMacros.IsValid` _hitcomponent
      (:`Is Valid`
        (return (and (== _hitactor (`local.InstigatorActor`)) (`|EnumEquality` (`PrimitiveComponent.GetCollisionObjectType` _hitcomponent) "ECC_GameTraceChannel1"))))
      (:`Is Not Valid`
        (return false)))
    (else
      (return false))))