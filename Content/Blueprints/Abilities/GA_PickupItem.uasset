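; Pickup action that turns the owning character toward the instigator and plays a grab-from-floor montage, startable only while moving on ground.
; An async turn-in-place through the TurnInPlaceComponent leads into the montage, whose notifies send an Action.Interacting gameplay event.
; The action finishes when the montage completes or is interrupted, and ending it stops the montage.
; Item destruction and inventory logic are unconnected placeholders.
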(event `self.ReceiveActionActivated`
  (bind (_ascharacter _bsuccess) (cast `Character` (`ActorComponent.GetOwner` (`self.OwnerComponent`)) :!pure true))
  (bind _output_get (set `self.TIPComponent` (`Actor.GetComponentByClass` (`ActorComponent.GetOwner` (`self.OwnerComponent`)) "/Script/StealthGame.TurnInPlaceComponent")))
  (set `self.OwnerCharacter` _ascharacter)
  (if (and (`KismetSystemLibrary.IsValid` _output_get) _bsuccess)
    (`AsyncTurnInPlace.AsyncTurnInPlace` (`self.TIPComponent`) (`KismetMathLibrary.Conv_VectorToRotator` (`KismetMathLibrary.GetDirectionUnitVector` (`Actor.K2_GetActorLocation` (`ActorComponent.GetOwner` (`self.OwnerComponent`))) (`Actor.K2_GetActorLocation` (`self.Instigator`))))
      (:`OnCompleted`
        (if (not (`self.IsCancelled`))
          (`|PlayMontage` (`Character.Mesh` (`self.OwnerCharacter`)) "/Game/Animations/Mixamo/UnarmedGrabTorchFromFloor_UE_Montage.UnarmedGrabTorchFromFloor_UE_Montage"
            (:`OnCompleted`
              (`self.FinishAction` :!label _label))
            (:`OnInterrupted`
              (goto _label))
            (:`OnNotifyBegin`
              (`ISGTagEventInterface.SendGameplayEvent2` (`self.OwnerComponent`) (struct :`TagName` "Action.Interacting") :!label _label_2))
            (:`OnNotifyEnd`
              (goto _label_2))))))
    (else
      (`self.FinishAction`))))

(event `self.ReceiveActionEnded`
  (set `self.IsCancelled` true)
  (`Character.StopAnimMontage` (cast `Character` (`self.OwnerActor`) :!pure true) "/Game/Animations/Mixamo/UnarmedGrabTorchFromFloor_UE_Montage.UnarmedGrabTorchFromFloor_UE_Montage"))

(fn `ReceiveCanStart`
  (params (NewActionData :type "GameplayActionData Structure (by ref)") (OwnerComp :type "SGameplayActionComponent Object Reference"))
  (returns (ReturnValue :type Boolean))
  (return (`NavMovementComponent.IsMovingOnGround` (`Actor.GetComponentByClass` (`self.OwnerActor`) "/Script/Engine.CharacterMovementComponent"))))