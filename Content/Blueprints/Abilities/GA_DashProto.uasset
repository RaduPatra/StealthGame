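; Prototype dash action that propels the owning character forward with a jet-boost montage while changing global time dilation.
; Start saves rotation rate and time dilation, applies dash values and switches to Flying.
; Tick drives forward velocity without root motion during the loop section until time expires, then restores Walking and montage root motion and jumps to the end section.
; Time dilation resets directly or lerps to 1.0 using dilation-compensated time; camera lag handling is unwired.
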(event `self.ReceiveActionActivated`
  (`self.Initialize`)
  (`self.StartDash`))

(event `StartDash`
  (`self.SetupDashStart`)
  (bind _notifyname (`|PlayMontage` (`self.Mesh`) "/Game/Animations/RobotPolice_JetBoost_DashForward_Montage_AI.RobotPolice_JetBoost_DashForward_Montage_AI")
    (:`OnCompleted`
      (`self.FinishAction`))
    (:`OnInterrupted`
      (`self.CancelAction`))
    (:`OnNotifyBegin`
      (`KismetSystemLibrary.PrintString` (`KismetStringLibrary.Conv_NameToString` _notifyname) :!label _label))
    (:`OnNotifyEnd`
      (goto _label))))

(event `self.ReceiveTickAction`
  (params (DeltaTime :type "Float (single-precision)"))
  (`self.UpdateDash` DeltaTime))

(event `UpdateDash`
  (params (DeltaSeconds :type "Float (double-precision)"))
  (`|ExecutionSequence`
    (:`then_0`
      (if (`self.IsCurrentMontageInSection` (`self.DashLoopSectionName`))
        (`self.DoDashLoop` DeltaSeconds)
        (if (not (> (`self.DashRemainingTime`) 0.0))
          (`self.StartEndingDash`))))
    (:`then_1`
      (`self.LerpTimeDilation` DeltaSeconds))))

(event `self.ReceiveActionEnded`
  (`self.EndDash`))

(fn `DisablePlayerCameraLag`
  (`/Engine/EditorBlueprintResources/StandardMacros.IsValid` (`self.Third Person Character`)))

(fn `DoDashLoop`
  (params (InputPin :type "Float (double-precision)"))
  (`AnimInstance.SetRootMotionMode` (`SkeletalMeshComponent.GetAnimInstance` (`self.Mesh`)) "IgnoreRootMotion")
  (set `MovementComponent.Velocity` (* (`Actor.GetActorForwardVector` (`self.OwnerActor`)) (`self.DashLoopSpeed`)) (`self.CharacterMovement`))
  (set `self.DashRemainingTime` (- (`self.DashRemainingTime`) InputPin)))

(fn `EndDash`
  (`self.DisablePlayerCameraLag`) ; This interpolates camera speed to 0 which prevents snapping when disabling it.\nwe have to do it in player class because dash ability lifespan could be shorter
  (if (not (`self.ShouldLerpTimeDilation`))
    (`self.SetTimeDilation` (`self.DefaultTimeDilation`)))
  (set `CharacterMovementComponent.RotationRate` (`self.RotationRateBeforeDash`) (`self.CharacterMovement`)))

(fn `Initialize`
  (bind _ascharacter (cast `Character` (`self.OwnerActor`)))
  (bind _output_get (set `self.OwnerCharacter` _ascharacter))
  (set `self.Mesh` (`Character.Mesh` _output_get))
  (set `self.CharacterMovement` (`Character.CharacterMovement` _ascharacter))
  (set `self.CameraBoom` (`Actor.GetComponentByClass` (`self.OwnerActor`) "/Script/Engine.SpringArmComponent"))
  (bind _asbp_third_person_character (cast `/Game/Blueprints/BP_ThirdPersonCharacter` (`self.OwnerActor`)))
  (set `self.Third Person Character` _asbp_third_person_character))

(fn `IsCurrentMontageInSection`
  (params (SectionName :type Name))
  (returns (ReturnValue :type Boolean))
  (return (== SectionName (`AnimInstance.Montage_GetCurrentSection` (`SkeletalMeshComponent.GetAnimInstance` (`self.Mesh`)) (`Character.GetCurrentMontage` (`self.OwnerCharacter`))))))

(fn `LerpTimeDilation`
  (params (InputPin :type "Float (double-precision)"))
  (if (`self.IsLerpingTimeDilation`)
    (set `self.CurrentTimeDilation` (`KismetMathLibrary.Lerp` (`self.DashTimeDilation`) 1.0 (/ (`self.CurrentLoopingSeconds`) (`self.TimeDilationLerpTime`))))
    (set `self.CurrentLoopingSeconds` (+ (`self.CurrentLoopingSeconds`) (* InputPin (/ 1.0 (`self.CurrentTimeDilation`)))))
    (`self.SetTimeDilation` (`self.CurrentTimeDilation`))
    (if (>= (`GameplayStatics.GetGlobalTimeDilation`) 1.0)
      (set `self.IsLerpingTimeDilation` false))))

(fn `SetTimeDilation`
  (params (TimeDilation :type "Float (single-precision)"))
  (`/Engine/EditorBlueprintResources/StandardMacros.IsValid` (`self.Third Person Character`)
    (:`Is Valid`
      (`GameplayStatics.SetGlobalTimeDilation` TimeDilation))))

(fn `SetupDashStart`
  (set `self.RotationRateBeforeDash` (`CharacterMovementComponent.RotationRate` (`self.CharacterMovement`)))
  (set `self.DefaultTimeDilation` (`GameplayStatics.GetGlobalTimeDilation`))
  (set `self.DashRemainingTime` (`self.DashTime`))
  (set `CharacterMovementComponent.RotationRate` (`self.DashRotationRate`) (`self.CharacterMovement`))
  (set `self.CurrentLoopingSeconds` 0.0)
  (set `self.IsLerpingTimeDilation` false)
  (bind _output_get (set `self.CurrentTimeDilation` (`self.DashTimeDilation`)))
  (`self.SetTimeDilation` _output_get)
  (`CharacterMovementComponent.SetMovementMode` (`self.CharacterMovement`) "MOVE_Flying" 0)
  (`/Engine/EditorBlueprintResources/StandardMacros.IsValid` (`self.Third Person Character`)))

(fn `StartEndingDash`
  (`CharacterMovementComponent.SetMovementMode` (`self.CharacterMovement`) "MOVE_Walking" 0)
  (`AnimInstance.SetRootMotionMode` (`SkeletalMeshComponent.GetAnimInstance` (`self.Mesh`)) "RootMotionFromMontagesOnly")
  (`AnimInstance.Montage_JumpToSection` (`SkeletalMeshComponent.GetAnimInstance` (`self.Mesh`)) (`self.DashEndSectionName`) (`Character.GetCurrentMontage` (`self.OwnerCharacter`)))
  (if (`self.ShouldLerpTimeDilation`)
    (set `self.IsLerpingTimeDilation` true)
    (else
      (`self.SetTimeDilation` (`self.DefaultTimeDilation`)))))