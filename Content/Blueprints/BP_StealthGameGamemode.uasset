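; Stealth game mode that tracks registered NPC controllers and serializes their EQS chase-point queries so only one runs at a time.
; CalcInfluence inserts each requester once at the front of a queue, which is served from the back in first-in, first-out order.
; When EQS_ChasePoints finishes, it prints item scores, writes the first result to that NPC's move-to blackboard key and starts the next queued query.
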(event `self.ReceiveBeginPlay`)

(event `CalcInfluence`
  (params (QuerierController :type "AIController Object Reference"))
  (if (> (`KismetArrayLibrary.Array_Length` (`self.NPCsToQueryForQueue`)) 1)
    _
    (else
      _))
  (if (not (`KismetArrayLibrary.Array_Contains` (`self.NPCsToQueryForQueue`) QuerierController))
    (`KismetArrayLibrary.Array_Insert` (`self.NPCsToQueryForQueue`) QuerierController)
    (`self.RunQuery` (`|GetArrayItem` (`self.NPCsToQueryForQueue`) (`KismetArrayLibrary.Array_LastIndex` (`self.NPCsToQueryForQueue`))))))

(event `RunQuery`
  (params (Querier :type "AIController Object Reference"))
  (`/Engine/EditorBlueprintResources/StandardMacros.IsValid` (`self.AICurrentlyBeingQuerried`)
    (:`Is Not Valid`
      (bind _output_get (set `self.AICurrentlyBeingQuerried` Querier))
      (`self.RunQueryFromQueue` _output_get))))

(event `RunQueryFromQueue`
  (params (Querier :type "AIController Object Reference"))
  (bind _returnvalue (`EnvQueryManager.RunEQSQuery` "/Game/Blueprints/AI/EQS/EQS_ChasePoints.EQS_ChasePoints" Querier "AllMatching"))
  (set `self.QueryRunning` true)
  (add `EnvQueryInstanceBlueprintWrapper.OnQueryFinishedEvent` _returnvalue (delegate `QueryFinished`)))

(event `QueryFinished`
  (params (QueryInstance :type "EnvQueryInstanceBlueprintWrapper Object Reference") (QueryStatus :type "EEnvQueryStatus Enum" :default "Processing"))
  (bind _npcstoqueryforqueue (`self.NPCsToQueryForQueue`))
  (bind _output (`|GetArrayItem` (`self.NPCsToQueryForQueue`) (`KismetArrayLibrary.Array_LastIndex` (`self.NPCsToQueryForQueue`))))
  (bind _resultlocations (`EnvQueryInstanceBlueprintWrapper.GetQueryResultsAsLocations` QueryInstance))
  (for (_ _array_index) _resultlocations
    (`KismetSystemLibrary.PrintString` (`KismetStringLibrary.Conv_DoubleToString` (`EnvQueryInstanceBlueprintWrapper.GetItemScore` QueryInstance _array_index))))
  (`BlackboardComponent.SetValueAsVector` (`AIBlueprintHelperLibrary.GetBlackboard` (`self.AICurrentlyBeingQuerried`)) (`self.MoveToLocationKey`) (`|GetArrayItem` _resultlocations))
  (`KismetArrayLibrary.Array_Remove` _npcstoqueryforqueue (`KismetArrayLibrary.Array_LastIndex` _npcstoqueryforqueue))
  (if (> (`KismetArrayLibrary.Array_Length` (`self.NPCsToQueryForQueue`)) 0)
    (set `self.AICurrentlyBeingQuerried` _output)
    (`self.RunQueryFromQueue` _output)
    (else
      (set `self.AICurrentlyBeingQuerried` (`self.NullController`)))))

(event `RegisterNPCs`
  (params (Controller :type "AIController Object Reference"))
  (`KismetArrayLibrary.Array_AddUnique` (`self.AllNPCs`) Controller))

(event `UnregisterNPC`
  (params (Controller :type "AIController Object Reference"))
  (`KismetArrayLibrary.Array_RemoveItem` (`self.AllNPCs`) Controller))

(fn `UserConstructionScript`)