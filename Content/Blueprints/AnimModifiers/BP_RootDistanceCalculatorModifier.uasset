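; BP_RootDistanceCalculatorModifier is an animation modifier that measures how far the root bone travels across an animation sequence.
; On apply, it reads the root bone location at the first and last frames, then logs both positions and their straight-line 2D distance.
; It leaves the sequence unchanged: the distance-curve writing nodes are disconnected, and revert does nothing.
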(event `self.OnApply`
  (params (AnimationSequence :type "AnimSequence Object Reference"))
  (set `self.Animation Sequence` AnimationSequence)
  (set `self.NumFrames` (`AnimationBlueprintLibrary.GetNumFrames` (`self.Animation Sequence`)))
  (set `self.StartPoseLocation` (.location (`AnimationBlueprintLibrary.GetBonePoseForFrame` (`self.Animation Sequence`) (`self.RootBoneName`))))
  (set `self.EndPoseLocation` (.location (`AnimationBlueprintLibrary.GetBonePoseForFrame` (`self.Animation Sequence`) (`self.RootBoneName`) (`self.NumFrames`))))
  (`KismetSystemLibrary.LogString` (`KismetStringLibrary.Concat_StrStr` "Start " (`KismetStringLibrary.Conv_VectorToString` (`self.StartPoseLocation`)) "End" (`KismetStringLibrary.Conv_VectorToString` (`self.EndPoseLocation`)) "Distance" (`KismetStringLibrary.Conv_DoubleToString` (`KismetMathLibrary.Vector_Distance2D` (`self.StartPoseLocation`) (`self.EndPoseLocation`))))))

(event `self.OnRevert`
  (params (AnimationSequence :type "AnimSequence Object Reference")))