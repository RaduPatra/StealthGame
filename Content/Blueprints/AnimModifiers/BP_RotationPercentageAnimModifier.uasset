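; Animation modifier that bakes a normalized 0-to-1 progress curve from an animation sequence's rotation curve.
; On apply, it removes any existing normalized curve and reads the rotation curve's key times and values.
; It remaps each value with a clamped range from first key to last, then writes the results to a new curve at the same times.
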(event `self.OnApply`
  (params (AnimationSequence :type "AnimSequence Object Reference"))
  (bind _distancecurvevalues (`self.DistanceCurveValues`))
  (bind _output_get (set `self.Animation Sequence` AnimationSequence))
  (`AnimationBlueprintLibrary.RemoveCurve` _output_get (`self.Normalized Curve Name`))
  (bind (_times _values) (`AnimationBlueprintLibrary.GetFloatKeys` _output_get (`self.RotationCurveName`)))
  (set `self.DistanceCurveTimes` _times)
  (set `self.DistanceCurveValues` _values)
  (set `self.FirstCurveValue` (`|GetArrayItem` (`self.DistanceCurveValues`)))
  (set `self.LastCurveValue` (`|GetArrayItem` _distancecurvevalues (- (`KismetArrayLibrary.Array_Length` _distancecurvevalues) 1)))
  (for _array_element (`self.DistanceCurveValues`)
    (`KismetArrayLibrary.Array_Add` (`self.NormalizedCurveValues`) (`KismetMathLibrary.MapRangeClamped` _array_element (`self.FirstCurveValue`) (`self.LastCurveValue`) 0.0 1.0)))
  (`AnimationBlueprintLibrary.AddCurve` (`self.Animation Sequence`) (`self.Normalized Curve Name`))
  (`AnimationBlueprintLibrary.AddFloatCurveKeys` (`self.Animation Sequence`) (`self.Normalized Curve Name`) (`self.DistanceCurveTimes`) (`self.NormalizedCurveValues`)))