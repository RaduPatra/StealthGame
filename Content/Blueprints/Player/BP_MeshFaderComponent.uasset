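; BP_MeshFaderComponent is a player component for handling meshes that block the camera's view of its owner.
; OccludeMeshes runs a multi line trace for WorldStatic objects from the camera manager to the owner, then passes hits to ProcessHitResults, defined outside this graph.
; It prints a warning when the owner is not a player-controlled pawn.
; BeginPlay is empty and the looping timer that would call OccludeMeshes is disconnected.
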(event `self.ReceiveBeginPlay`)

(event `OccludeMeshes`
  (bind _aspawn (cast `Pawn` (`self.GetOwner`))
    (:`then`
      (bind _asplayer_controller (cast `PlayerController` (`Pawn.GetController` _aspawn))
        (:`then`
          (bind _outhits (`KismetSystemLibrary.LineTraceMultiForObjects` (`PlayerCameraManager.GetCameraLocation` (`PlayerController.PlayerCameraManager` _asplayer_controller)) (`Actor.K2_GetActorLocation` (`self.GetOwner`)) (`|MakeArray` "ObjectTypeQuery1" "ObjectTypeQuery1" "ObjectTypeQuery1" "ObjectTypeQuery1" "ObjectTypeQuery1" "ObjectTypeQuery1" "ObjectTypeQuery1" "ObjectTypeQuery1" "ObjectTypeQuery1" :!type "EObjectTypeQuery Enum")))
          (`self.ProcessHitResults` _outhits))
        (:`CastFailed`
          (`KismetSystemLibrary.PrintString` "Fader needs to be on player" :!label _label))))
    (:`CastFailed`
      (goto _label))))