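; Test interactable actor with a sparks effect that the player toggles on and off, reporting a noise event when it turns on.
; Interact branches on the interactor's gameplay tag, but its NPC branch only checks whether sparks are active.
; ToggleSparks and TurnOffSparks provide separate player and AI actions.
; Much is unfinished: turn-in-place, montage and behavior-tree logic is disconnected, and several interaction functions are empty stubs.
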(event `self.ReceiveBeginPlay`)

(event `CustomEvent_1`
  (params (Interactor :type "SInteractor Object Reference")))

(event `self.P_Sparks.OnComponentActivated`
  (params (Component :type "ActorComponent Object Reference") (bReset :type Boolean))
  (set `self.bSparksActive` true))

(event `self.P_Sparks.OnComponentDeactivated`
  (params (Component :type "ActorComponent Object Reference"))
  (set `self.bSparksActive` false))

(event `self.StartInteract`
  (params (Interactor :type "SInteractor Object Reference")))

(fn `CanInteract`
  (params (Interactor :type "SInteractor Object Reference"))
  (returns (ReturnValue :type "InteractResult Structure") (ReturnValue :type Boolean)))

(fn `GetInteractableType`
  (returns (ReturnValue :type "GameplayTag Structure"))
  (return))

(fn `Interact`
  (params (Interactor :type "SInteractor Object Reference"))
  (locals (InteractorObj :type "SInteractor Object Reference"))
  (bind _p_sparks (`self.P_Sparks`))
  (bind _output_get (set `local.InteractorObj` Interactor))
  (`|SwitchGameplayTag` (`SInteractor.GetInteractorTag` _output_get)
    (:`Character.Player`
      (`ActorComponent.ToggleActive` _p_sparks)
      (if (`ActorComponent.IsActive` _p_sparks)
        (`AISense_Hearing.ReportNoiseEvent` (`SceneComponent.K2_GetComponentLocation` (`self.BestInteractLocation`)) 1.0 self)
        (`SInteractor.FinishInteract` (`local.InteractorObj`) false)))
    (:`Character.NPC`
      (if (`ActorComponent.IsActive` (`self.P_Sparks`))
        _))))

(fn `ToggleSparks`
  (bind _p_sparks (`self.P_Sparks`))
  (`ActorComponent.ToggleActive` _p_sparks)
  (if (`ActorComponent.IsActive` _p_sparks)
    (`AISense_Hearing.ReportNoiseEvent` (`SceneComponent.K2_GetComponentLocation` (`self.BestInteractLocation`)) 1.0 null)))

(fn `TryStartInteract`
  (params (Interactor :type "SInteractor Object Reference"))
  (returns (ReturnValue :type "InteractResult Structure"))
  (return))

(fn `TurnOffSparks`
  (`ActorComponent.Deactivate` (`self.P_Sparks`)))

(fn `UserConstructionScript`)